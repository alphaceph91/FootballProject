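; BP_Football is a kickable football actor that the player launches while inside its trigger box.
; Box overlap begin and end events enable and disable the actor's input for player 0, without filtering the overlapping actor.
; While enabled, IA_Kick applies a velocity-change impulse to the static mesh along the player controller's forward vector, scaled by Speed.
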(event `self.Box.OnComponentBeginOverlap`
  (params (OverlappedComponent :type "PrimitiveComponent Object Reference") (OtherActor :type "Actor Object Reference") (OtherComp :type "PrimitiveComponent Object Reference") (OtherBodyIndex :type Integer) (bFromSweep :type Boolean) (SweepResult :type "HitResult Structure (by ref)"))
  ;[1 1 1] Football Trigger Box
  (`self.EnableInput` (`GameplayStatics.GetPlayerController` 0)))

(event `self.Box.OnComponentEndOverlap`
  (params (OverlappedComponent :type "PrimitiveComponent Object Reference") (OtherActor :type "Actor Object Reference") (OtherComp :type "PrimitiveComponent Object Reference") (OtherBodyIndex :type Integer))
  ;[1 1 1] Football Trigger Box
  (`self.DisableInput` (`GameplayStatics.GetPlayerController` 0)))

(event `EnhancedInput|/Game/FootballGame/Framework/Input/IA_Kick`
  (params (ActionValue :type Boolean) (ElapsedSeconds :type "Float (double-precision)") (TriggeredSeconds :type "Float (double-precision)") (InputAction :type "InputAction Object Reference" :default "/Game/FootballGame/Framework/Input/IA_Kick.IA_Kick"))
  ;[1 1 1] Football Kick Logic
  (:`Started`
    (`PrimitiveComponent.AddImpulse` (`self.StaticMesh`) (* (`self.GetActorForwardVector` (`GameplayStatics.GetPlayerController` 0)) (`self.Speed`)) "None" true)))

(fn `UserConstructionScript`)