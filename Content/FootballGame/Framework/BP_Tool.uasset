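; BP_Tool is a construction-script placement tool that lines up copies of a chosen mesh from the actor's origin toward EndPoint.
; It fits as many whole Width steps as the distance allows and adds one local-space InstancedStaticMesh instance per step, rotated to face EndPoint.
; The offset term divides Width by zero, apparently leaving instances at whole-Width multiples.
; The event graph has no active logic.
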(fn `UserConstructionScript`
  (bind _width (`self.Width`))
  (bind _returnvalue (`KismetMathLibrary.FindLookAtRotation` (0.0 0.0 0.0) (`self.EndPoint`)))
  (`StaticMeshComponent.SetStaticMesh` (`self.InstancedStaticMesh`) (`self.MeshToSpawn`))
  (for _index (range 1 (+ (`KismetMathLibrary.FFloor` (/ (`KismetMathLibrary.VSize` (`self.EndPoint`)) (`self.Width`))) 1))
    (`InstancedStaticMeshComponent.AddInstance` (`self.InstancedStaticMesh`) (`KismetMathLibrary.MakeTransform` (* (- (* _index _width) (/ _width 0.0)) (`KismetMathLibrary.GetForwardVector` _returnvalue)) _returnvalue) false)))